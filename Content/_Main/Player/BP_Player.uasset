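; Player Blueprint that handles movement, jumping, moving allies, and summoning or enlisting units with mana.
; Enhanced Input events call inherited actions, with Tick moving allies while that input is held.
; The construction script registers mana and summon MVVM viewmodels in the global collection.
; Mana changes update the mana viewmodel, a change to the summoned unit template enters summoning mode, and health changes refresh the health bar widget.
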(event HealthChangedPercent(HealthComponent)
  (params (NewPercent :type Float%20%28single-precision%29))
  (CallFunction|UpdateHealthBarWidget NewPercent (Variables|Default|GetHealthBar)))

(event Custom|OnUnitTemplateBeingSummonedChanged
  (params (Object :type Object%20Object%20Reference) (Field :type Field%20Notification%20Id%20Structure))
  (Class|DefaultPlayer|EnterSummoningMode (Variables|/Game/_Main/Player/VM_Summon.VM_Summon_C|GetUnitTemplateBeingSummoned (Variables|Default|GetVM_Summon))))

(event Custom|OnManaChanged
  (params (NewValue :type Integer))
  (Default|SetCurrent (Variables|Default|GetVM_Mana) NewValue)
  (Default|SetMax (Variables|Default|GetVM_Mana) (Variables|Default|GetMaxMana)))

(event Input|EnhancedActionEvents|EnhancedInputActionIA_Move
  (params (ActionValue :type Vector%202D%20Structure) (ElapsedSeconds :type Float%20%28double-precision%29) (TriggeredSeconds :type Float%20%28double-precision%29) (InputAction :type Input%20Action%20Object%20Reference :default "/Game/_Main/Input/Actions/IA_Move.IA_Move"))
  (Class|DefaultPlayer|Move ActionValue))

(event Input|EnhancedActionEvents|EnhancedInputActionIA_Jump
  (params (ActionValue :type Boolean) (ElapsedSeconds :type Float%20%28double-precision%29) (TriggeredSeconds :type Float%20%28double-precision%29) (InputAction :type Input%20Action%20Object%20Reference :default "/Game/_Main/Input/Actions/IA_Jump.IA_Jump"))
  (Character|Jump))

(event Input|EnhancedActionEvents|EnhancedInputActionIA_MoveAllies
  (params (ActionValue :type Boolean) (ElapsedSeconds :type Float%20%28double-precision%29) (TriggeredSeconds :type Float%20%28double-precision%29) (InputAction :type Input%20Action%20Object%20Reference :default "/Game/_Main/Input/Actions/IA_MoveAllies.IA_MoveAllies"))
  (:Triggered
    (Variables|Default|SetIsMovingAllies true))
  (:Completed
    (Variables|Default|SetIsMovingAllies false)))

(event Input|EnhancedActionEvents|EnhancedInputActionIA_SummonAlly
  (params (ActionValue :type Boolean) (ElapsedSeconds :type Float%20%28double-precision%29) (TriggeredSeconds :type Float%20%28double-precision%29) (InputAction :type Input%20Action%20Object%20Reference :default "/Game/_Main/Input/Actions/IA_SummonAlly.IA_SummonAlly"))
  (Class|DefaultPlayer|SummonorEnlistUnit))

(event EventBeginPlay
  (EventDispatchers|BindEventtoManaChanged (EventDispatchers|CreateEvent :!event Custom|OnManaChanged))
  (Class|MVVMViewModelBase|AddFieldValueChangedDelegate (Variables|Default|GetVM_Summon) "(FieldName=\"UnitTemplateBeingSummoned\")" (EventDispatchers|CreateEvent :!event Custom|OnUnitTemplateBeingSummonedChanged)))

(event EventTick
  (params (DeltaSeconds :type Float%20%28single-precision%29))
  (if (Variables|Default|GetIsMovingAllies)
    (Class|DefaultPlayer|MoveAllies)))

(fn ConstructionScript
  (CallFunction|InitGlobalManaViewmodel)
  (CallFunction|InitGlobalSummonViewmodel))

(fn InitGlobalManaViewmodel
  (Variables|Default|GetVM_Mana
    (:then
      _)
    (:else
      (bind _returnvalue (Game|ConstructObjectfromClass self "/Game/_Main/Player/VM_Mana.VM_Mana_C" (Variables|Default|GetCurrentMana) (Variables|Default|GetMaxMana)))
      (Variables|Default|SetVM_Mana _returnvalue)))
  (Class|MVVMViewModelCollectionObject|AddViewModelInstance (Class|MVVMGameSubsystem|GetViewModelCollection (Subsystems|GetMVVMGameSubsystem)) (Utilities|Struct|MakeMVVMViewModelContext "/Game/_Main/Player/VM_Mana.VM_Mana_C" "VM_Mana") (Variables|Default|GetVM_Mana)))

(fn InitGlobalSummonViewmodel
  (Variables|Default|GetVM_Summon
    (:then
      _)
    (:else
      (bind _returnvalue (Game|ConstructObjectfromClass self "/Game/_Main/Player/VM_Summon.VM_Summon_C" (Variables|Default|GetUnitTemplates)))
      (Variables|Default|SetVM_Summon _returnvalue)))
  (Class|MVVMViewModelCollectionObject|AddViewModelInstance (Class|MVVMGameSubsystem|GetViewModelCollection (Subsystems|GetMVVMGameSubsystem)) (Utilities|Struct|MakeMVVMViewModelContext "/Game/_Main/Player/VM_Summon.VM_Summon_C" "VM_Summon") (Variables|Default|GetVM_Summon)))